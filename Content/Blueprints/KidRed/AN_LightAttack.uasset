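; Animation notify for KidRed's light attack that deals melee damage when it fires in the animation.
; On authority only, it runs a box overlap at the render component's right-hand socket, ignoring the attacker.
; For overlapped GasPaperCharacters on the opposite side, decided by comparing the Type.Enemy tag, it sends a GAS Event.Damage gameplay event with a fixed magnitude.
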(fn `OnReceiveNotify`
  (params (OwningInstance :type "PaperZDAnimInstance Object Reference"))
  (bind _returnvalue (`PaperZDAnimInstance.GetOwningActor` OwningInstance))
  (`/Engine/EditorBlueprintResources/StandardMacros.IsValid` OwningInstance
    (:`Is Valid`
      (if (`Actor.HasAuthority` _returnvalue)
        (bind _outactors (`KismetSystemLibrary.BoxOverlapActors` (`SceneComponent.GetSocketLocation` (`self.SequenceRenderComponent`) "RightHandSocket") (`self.Extent`) (`|MakeArray` "ObjectTypeQuery7" "ObjectTypeQuery3" :!type "EObjectTypeQuery Enum") null (`|MakeArray` _returnvalue)))
        (for _array_element _outactors
          (bind _asgas_paper_character (cast `GasPaperCharacter` (`PaperZDAnimInstance.GetOwningActor` OwningInstance)))
          (bind _asgas_paper_character_2 (cast `GasPaperCharacter` _array_element))
          (bind _returnvalue_2 (`GasPaperCharacter.GetMyAbilitySystemComponent` _asgas_paper_character_2))
          (if (!= (`GameplayTagAssetInterface.HasMatchingGameplayTag` _returnvalue_2 (struct :`TagName` "Type.Enemy")) (`GameplayTagAssetInterface.HasMatchingGameplayTag` (`GasPaperCharacter.GetMyAbilitySystemComponent` _asgas_paper_character) (struct :`TagName` "Type.Enemy")))
            (bind _returnvalue_3 (`ActorComponent.GetOwner` _returnvalue_2))
            (`AbilitySystemBlueprintLibrary.SendGameplayEventToActor` _returnvalue_3 (struct :`TagName` "Event.Damage") (make `GameplayEventData` (struct :`TagName` "Event.Damage") _asgas_paper_character _returnvalue_3 null null (struct) (struct) (struct) 20.0))))))))